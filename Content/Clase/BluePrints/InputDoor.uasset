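; InputDoor is a door Blueprint that swings open when the player's third-person character enters its trigger and closes when it leaves.
; Overlap events on OpenDoorCollider, filtered by a cast to BP_ThirdPersonCharacter, play or reverse the OpenDoor timeline.
; The timeline's interpolated value, multiplied by MaxRotation, sets the relative yaw of SMDoor.
; BeginPlay enables player input, though the event graph handles no input events.
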(event `self.ReceiveBeginPlay`
  (`self.EnableInput` (`GameplayStatics.GetPlayerController` 0)))

(event `InputAction|OpenDoor`
  (params (Key :type "Key Structure")))

(event `self.OpenDoorCollider.OnComponentBeginOverlap`
  (params (OverlappedComponent :type "PrimitiveComponent Object Reference") (OtherActor :type "Actor Object Reference") (OtherComp :type "PrimitiveComponent Object Reference") (OtherBodyIndex :type Integer) (bFromSweep :type Boolean) (SweepResult :type "HitResult Structure (by ref)"))
  ;[1 1 1] ColliderDeLaPuerta
  ;[1 1 1] Comprobador del personaje
  (cast `/Game/ThirdPerson/Blueprints/BP_ThirdPersonCharacter` OtherActor)
  (bind (_direction _doorrotationinterpolatedvalue) (`Timeline|OpenDoor` :!label _label)
    (:`Update`
      ;[1 1 1] Rotacion
      (`SceneComponent.K2_SetRelativeRotation` (`self.SM_Door`) (`KismetMathLibrary.MakeRotator` 0.0 0.0 (* _doorrotationinterpolatedvalue (`self.MaxRotation`))) false false))))

(event `self.OpenDoorCollider.OnComponentEndOverlap`
  (params (OverlappedComponent :type "PrimitiveComponent Object Reference") (OtherActor :type "Actor Object Reference") (OtherComp :type "PrimitiveComponent Object Reference") (OtherBodyIndex :type Integer))
  ;[1 1 1] ColliderDeLaPuerta
  ;[1 1 1] Comprobador del personaje
  (cast `/Game/ThirdPerson/Blueprints/BP_ThirdPersonCharacter` OtherActor)
  (goto _label :!via `Reverse`))

(fn `UserConstructionScript`)