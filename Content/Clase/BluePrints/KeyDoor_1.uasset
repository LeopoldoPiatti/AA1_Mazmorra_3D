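; Key-locked door Blueprint that the player swings open and closed with the OpenDoor input.
; The collider's overlap with BP_ThirdPersonCharacter opens a gate, so input only works nearby.
; A locked door with NeedSpecificKey set spends one of the character's Keys and stays unlocked.
; Once unlocked, a FlipFlop alternately plays and reverses a Timeline that scales the door mesh's yaw by MaxRotation.
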(event `self.ReceiveBeginPlay`
  (`self.EnableInput` (`GameplayStatics.GetPlayerController` 0)))

(event `InputAction|OpenDoor` :consume false
  (params (Key :type "Key Structure"))
  (:`Pressed`
    (`/Engine/EditorBlueprintResources/StandardMacros.Gate` true :!label _label
      (:`Exit`
        (if (`self.UnLocked`)
          (`/Engine/EditorBlueprintResources/StandardMacros.FlipFlop` :!label _label_2
            (:`A`
              (bind (_direction _doorrotationinterpolatedvalue) (`Timeline|Timeline` :!label _label_3)
                (:`Update`
                  ;[1 1 1] Rotacion
                  (`SceneComponent.K2_SetRelativeRotation` (`self.SM_Door`) (`KismetMathLibrary.MakeRotator` 0.0 0.0 (* _doorrotationinterpolatedvalue (`self.MaxRotation`))) false false))))
            (:`B`
              (goto _label_3 :!via `Reverse`)))
          (elif (`self.NeedSpecificKey`)
            (bind _keys (`/Game/ThirdPerson/Blueprints/BP_ThirdPersonCharacter.Keys` (stale `self.OpenDoorCollider.OnComponentBeginOverlap` _asbp_third_person_character)))
            (if (>= _keys 1)
              (`/Engine/EditorBlueprintResources/StandardMacros.DecrementInt` _keys
                (:`  `
                  (set `self.UnLocked` true)
                  (goto _label_2))))))))))

(event `self.OpenDoorCollider.OnComponentBeginOverlap`
  (params (OverlappedComponent :type "PrimitiveComponent Object Reference") (OtherActor :type "Actor Object Reference") (OtherComp :type "PrimitiveComponent Object Reference") (OtherBodyIndex :type Integer) (bFromSweep :type Boolean) (SweepResult :type "HitResult Structure (by ref)"))
  ;[1 1 1] ColliderDeLaPuerta
  ;[1 1 1] Comprobador del personaje
  (bind _asbp_third_person_character (cast `/Game/ThirdPerson/Blueprints/BP_ThirdPersonCharacter` OtherActor))
  (goto _label :!via `Open`))

(event `self.OpenDoorCollider.OnComponentEndOverlap`
  (params (OverlappedComponent :type "PrimitiveComponent Object Reference") (OtherActor :type "Actor Object Reference") (OtherComp :type "PrimitiveComponent Object Reference") (OtherBodyIndex :type Integer))
  ;[1 1 1] ColliderDeLaPuerta
  ;[1 1 1] Comprobador del personaje
  (cast `/Game/ThirdPerson/Blueprints/BP_ThirdPersonCharacter` OtherActor)
  (goto _label :!via `Close`))

(fn `UserConstructionScript`)