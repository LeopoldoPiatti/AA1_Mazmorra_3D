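; Key is a pickup actor that the player character collects on overlap to open doors.
; On BeginPlay, a linked KeyDoorSpe door, if valid, is flagged as needing a specific key.
; When BP_ThirdPersonCharacter enters the Collision component, the key unlocks that linked door, or increments the character's generic Keys count if none is linked, then destroys itself.
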(event `self.ReceiveBeginPlay`
  (bind _keydoorspe (`self.KeyDoorSpe`))
  (`/Engine/EditorBlueprintResources/StandardMacros.IsValid` _keydoorspe
    (:`Is Valid`
      (set `/Game/Clase/BluePrints/KeyDoor_1.NeedSpecificKey` true _keydoorspe))))

(event `self.Collision.OnComponentBeginOverlap`
  (params (OverlappedComponent :type "PrimitiveComponent Object Reference") (OtherActor :type "Actor Object Reference") (OtherComp :type "PrimitiveComponent Object Reference") (OtherBodyIndex :type Integer) (bFromSweep :type Boolean) (SweepResult :type "HitResult Structure (by ref)"))
  (bind _keydoorspe (`self.KeyDoorSpe`))
  (bind _asbp_third_person_character (cast `/Game/ThirdPerson/Blueprints/BP_ThirdPersonCharacter` OtherActor))
  (`/Engine/EditorBlueprintResources/StandardMacros.IsValid` _keydoorspe
    (:`Is Valid`
      (set `/Game/Clase/BluePrints/KeyDoor_1.UnLocked` true _keydoorspe))
    (:`Is Not Valid`
      (`/Engine/EditorBlueprintResources/StandardMacros.IncrementInt` (`/Game/ThirdPerson/Blueprints/BP_ThirdPersonCharacter.Keys` _asbp_third_person_character)
        (:`  `
          _))))
  (`self.K2_DestroyActor`))

(fn `UserConstructionScript`)