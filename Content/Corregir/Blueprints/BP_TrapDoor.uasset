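; Trap door actor that slides its floor half when the matching player character enters the blue or red collider.
; Each collider casts to its own character class and plays a separate timeline, which shakes nearby cameras while moving the floor.
; Each update adds MaxLocation, scaled by the timeline value, to the floor's current relative location with sweep, so movement accumulates.
; A third collider zeroes an entering duck's velocity and stops its mesh animation.
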(event `self.Collider Blue.OnComponentBeginOverlap`
  (params (OverlappedComponent :type "PrimitiveComponent Object Reference") (OtherActor :type "Actor Object Reference") (OtherComp :type "PrimitiveComponent Object Reference") (OtherBodyIndex :type Integer) (bFromSweep :type Boolean) (SweepResult :type "HitResult Structure (by ref)"))
  (bind _floorhalf (`self.FloorHalf`))
  ;[1 1 1] Collider BLue
  ;[1 1 1] Comprobador del personaje
  (cast `/Game/Corregir/ThirdPerson/Blueprints/BP_TPC_NB_1` OtherActor)
  ;[1 1 1] Set Location
  (bind (_direction _doorslide) (`Timeline|DoorSlide`)
    (:`Update`
      (`SceneComponent.K2_SetRelativeLocation` _floorhalf (+ (`SceneComponent.RelativeLocation` _floorhalf) (* (`self.MaxLocation`) _doorslide)) true false)
      (`GameplayStatics.PlayWorldCameraShake` "/Game/Corregir/Blueprints/BP_CameraShake.BP_CameraShake_C" (`self.K2_GetActorLocation`) 0.0 500.0))))

(event `self.Collider Red.OnComponentBeginOverlap`
  (params (OverlappedComponent :type "PrimitiveComponent Object Reference") (OtherActor :type "Actor Object Reference") (OtherComp :type "PrimitiveComponent Object Reference") (OtherBodyIndex :type Integer) (bFromSweep :type Boolean) (SweepResult :type "HitResult Structure (by ref)"))
  (bind _floorhalf (`self.FloorHalf`))
  ;[1 1 1] Collider Red
  ;[1 1 1] Comprobador del personaje
  (cast `/Game/Corregir/ThirdPerson/Blueprints/BP_TPC_NR_2` OtherActor)
  ;[1 1 1] Set Location
  (bind (_direction _doorslide) (`Timeline|Timeline`)
    (:`Update`
      (`SceneComponent.K2_SetRelativeLocation` _floorhalf (+ (`SceneComponent.RelativeLocation` _floorhalf) (* (`self.MaxLocation`) _doorslide)) true false)
      (`GameplayStatics.PlayWorldCameraShake` "/Game/Corregir/Blueprints/BP_CameraShake.BP_CameraShake_C" (`self.K2_GetActorLocation`) 0.0 500.0))))

(event `self.DuckCollider.OnComponentBeginOverlap`
  (params (OverlappedComponent :type "PrimitiveComponent Object Reference") (OtherActor :type "Actor Object Reference") (OtherComp :type "PrimitiveComponent Object Reference") (OtherBodyIndex :type Integer) (bFromSweep :type Boolean) (SweepResult :type "HitResult Structure (by ref)"))
  ;[1 1 1] Duck Collision
  (bind _asbp_duck_v2 (cast `/Game/Corregir/Blueprints/BP_DuckV2` OtherActor))
  (set `/Game/Corregir/Blueprints/BP_DuckV2.Velocity` 0.0 _asbp_duck_v2)
  (`SkeletalMeshComponent.Stop` (`Character.Mesh` _asbp_duck_v2)))

(fn `UserConstructionScript`)