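; BP_SpeedObjV2 is a spinning, time-limited pickup that adds to the player's blue collectable count.
; When ColliderBlue overlaps a BP_TPC_NB_1, it increments that actor's CollectablesBlue and destroys itself.
; An uncollected pickup destroys itself after ChangeDuration, counted from BeginPlay.
; Tick yaws the ShurikenLow component by Velocity scaled with DeltaSeconds, keeping the spin frame-rate independent.
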(event `self.ReceiveBeginPlay`
  ;[1 1 1] Color Set and Specific Item
  (`KismetSystemLibrary.Delay` (`self.ChangeDuration`))
  (`self.K2_DestroyActor`))

(event `self.Collider Blue.OnComponentBeginOverlap`
  (params (OverlappedComponent :type "PrimitiveComponent Object Reference") (OtherActor :type "Actor Object Reference") (OtherComp :type "PrimitiveComponent Object Reference") (OtherBodyIndex :type Integer) (bFromSweep :type Boolean) (SweepResult :type "HitResult Structure (by ref)"))
  ;[1 1 1] Item Collection
  (bind _asbp_tpc_nb_1 (cast `/Game/Corregir/ThirdPerson/Blueprints/BP_TPC_NB_1` OtherActor))
  (set `/Game/Corregir/ThirdPerson/Blueprints/BP_TPC_NB_1.CollectablesBlue` (+ (`/Game/Corregir/ThirdPerson/Blueprints/BP_TPC_NB_1.CollectablesBlue` _asbp_tpc_nb_1) 1) _asbp_tpc_nb_1)
  (`self.K2_DestroyActor`))

(event `self.ReceiveTick`
  (params (DeltaSeconds :type "Float (single-precision)"))
  ;[1 1 1] Rotation
  (`SceneComponent.K2_AddLocalRotation` (`self.Shuriken_low`) (`KismetMathLibrary.MakeRotator` 0.0 0.0 (* DeltaSeconds (`self.Velocity`))) false false))

(fn `UserConstructionScript`)