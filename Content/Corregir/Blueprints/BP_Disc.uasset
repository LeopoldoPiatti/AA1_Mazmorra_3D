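; BP_Disc is a spinning, moving disc obstacle that sends either of two player characters back to a restart position on overlap.
; Tick rotates the disc by Velocity, while the Construction Script gives InterpToMovement two relative control points, the origin and Location.
; A box overlap casts to each character class and teleports it to its blue or red location, with a short delay only for BP_TPC_NB_1.
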(event `self.ReceiveTick`
  (params (DeltaSeconds :type "Float (single-precision)"))
  ;[1 1 1] Rotation
  (`SceneComponent.K2_AddLocalRotation` (`self.disc`) (`KismetMathLibrary.MakeRotator` 0.0 (* DeltaSeconds (`self.Velocity`))) false false))

(event `self.Box.OnComponentBeginOverlap`
  (params (OverlappedComponent :type "PrimitiveComponent Object Reference") (OtherActor :type "Actor Object Reference") (OtherComp :type "PrimitiveComponent Object Reference") (OtherBodyIndex :type Integer) (bFromSweep :type Boolean) (SweepResult :type "HitResult Structure (by ref)"))
  ;[1 1 1] Player detection and restart position
  (`|ExecutionSequence`
    (:`then_0`
      (bind _asbp_tpc_nb_1 (cast `/Game/Corregir/ThirdPerson/Blueprints/BP_TPC_NB_1` OtherActor))
      (`KismetSystemLibrary.Delay` 0.5)
      (`SceneComponent.K2_SetWorldLocation` (`Actor.RootComponent` _asbp_tpc_nb_1) (`self.New Location_Blue`) false true))
    (:`then_1`
      (bind _asbp_tpc_nr_2 (cast `/Game/Corregir/ThirdPerson/Blueprints/BP_TPC_NR_2` OtherActor))
      (`SceneComponent.K2_SetWorldLocation` (`Actor.RootComponent` _asbp_tpc_nr_2) (`self.New Location_Red`) false true))))

(fn `UserConstructionScript`
  (bind _interptomovement (`self.InterpToMovement`))
  ;[1 1 1] Disc Movement
  (`InterpToMovementComponent.AddControlPointPosition` _interptomovement (0.0 0.0 0.0) true)
  (`InterpToMovementComponent.AddControlPointPosition` _interptomovement (`self.Location`) true))