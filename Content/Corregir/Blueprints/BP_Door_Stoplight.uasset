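; BP_Door_Stoplight is a sliding door that opens when a blue or red player character arrives with enough collectables of its color.
; Each color's collider casts to its character class, checks that count against CollectableCuantity, then resets it to zero.
; Separate timelines per color move DoorSL by adding scaled MaxLocation to its current relative location each update, with sweep, while playing a world camera shake at the door.
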(event `self.Collider Blue.OnComponentBeginOverlap`
  (params (OverlappedComponent :type "PrimitiveComponent Object Reference") (OtherActor :type "Actor Object Reference") (OtherComp :type "PrimitiveComponent Object Reference") (OtherBodyIndex :type Integer) (bFromSweep :type Boolean) (SweepResult :type "HitResult Structure (by ref)"))
  (bind _door_sl (`self.Door_SL`))
  ;[1 1 1] Collider BLue
  ;[1 1 1] Comprobador del personaje
  (bind _asbp_tpc_nb_1 (cast `/Game/Corregir/ThirdPerson/Blueprints/BP_TPC_NB_1` OtherActor))
  ;[1 1 1] Door Logic
  (if (>= (`/Game/Corregir/ThirdPerson/Blueprints/BP_TPC_NB_1.CollectablesBlue` _asbp_tpc_nb_1) (`self.CollectableCuantity`))
    (set `/Game/Corregir/ThirdPerson/Blueprints/BP_TPC_NB_1.CollectablesBlue` 0 _asbp_tpc_nb_1)
    ;[1 1 1] Set Location
    (bind (_direction _doorslide) (`Timeline|DoorSlide`)
      (:`Update`
        (`SceneComponent.K2_SetRelativeLocation` _door_sl (+ (`SceneComponent.RelativeLocation` _door_sl) (* (`self.MaxLocation`) _doorslide)) true false)
        (`GameplayStatics.PlayWorldCameraShake` "/Game/Corregir/Blueprints/BP_CameraShake.BP_CameraShake_C" (`self.K2_GetActorLocation`) 0.0 500.0)))))

(event `self.Collider Red.OnComponentBeginOverlap`
  (params (OverlappedComponent :type "PrimitiveComponent Object Reference") (OtherActor :type "Actor Object Reference") (OtherComp :type "PrimitiveComponent Object Reference") (OtherBodyIndex :type Integer) (bFromSweep :type Boolean) (SweepResult :type "HitResult Structure (by ref)"))
  (bind _door_sl (`self.Door_SL`))
  ;[1 1 1] Collider Red
  ;[1 1 1] Comprobador del personaje
  (bind _asbp_tpc_nr_2 (cast `/Game/Corregir/ThirdPerson/Blueprints/BP_TPC_NR_2` OtherActor))
  ;[1 1 1] Door Logic
  (if (>= (`/Game/Corregir/ThirdPerson/Blueprints/BP_TPC_NR_2.CollectablesRed` _asbp_tpc_nr_2) (`self.CollectableCuantity`))
    (set `/Game/Corregir/ThirdPerson/Blueprints/BP_TPC_NR_2.CollectablesRed` 0 _asbp_tpc_nr_2)
    ;[1 1 1] Set Location
    (bind (_direction _doorslide) (`Timeline|Timeline`)
      (:`Update`
        (`SceneComponent.K2_SetRelativeLocation` _door_sl (+ (`SceneComponent.RelativeLocation` _door_sl) (* (`self.MaxLocation`) _doorslide)) true false)
        (`GameplayStatics.PlayWorldCameraShake` "/Game/Corregir/Blueprints/BP_CameraShake.BP_CameraShake_C" (`self.K2_GetActorLocation`) 0.0 500.0)))))

(fn `UserConstructionScript`)