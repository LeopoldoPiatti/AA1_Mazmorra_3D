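; Spinning shuriken collectable with a red light/green light rule for the blue and red ninja characters.
; Tick rotates it and flips its dynamic material tint and IsGreen every two seconds through a looping MultiGate.
; On green, ninjas alternately score as it teleports between two spots, and red's third pickup destroys it.
; On red, either overlap zeroes both counters, using references cached by each collider's cast, and returns it to start.
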(event `self.ReceiveBeginPlay`
  (bind _relativelocation (`SceneComponent.RelativeLocation` (`self.CollectableBase`)))
  ;[1 1 1] Color Set and Specific Item
  (bind _returnvalue (`PrimitiveComponent.CreateDynamicMaterialInstance` (`self.Shuriken_low`) 0 "/Game/Corregir/Materials/M_Stoplight.M_Stoplight" "None"))
  (bind _output_get (set `self.TintGlass` _returnvalue))
  (`MaterialInstanceDynamic.SetVectorParameterValue` _output_get "ColorBase" (struct :`G` 1.0 :`A` 1.0))
  (set `self.IsGreen` true)
  (set `self.OldLocation` _relativelocation)
  (set `self.NewLocation` (+ _relativelocation (-1000.0 0.0 0.0))))

(event `self.ColliderBlue.OnComponentBeginOverlap`
  (params (OverlappedComponent :type "PrimitiveComponent Object Reference") (OtherActor :type "Actor Object Reference") (OtherComp :type "PrimitiveComponent Object Reference") (OtherBodyIndex :type Integer) (bFromSweep :type Boolean) (SweepResult :type "HitResult Structure (by ref)"))
  ;[1 1 1] Item Collection Blue Ninja
  (bind _asbp_tpc_nb_1 (cast `/Game/Corregir/ThirdPerson/Blueprints/BP_TPC_NB_1` OtherActor))
  (if (`self.IsGreen`)
    (if (`self.ChangePlace`)
      (`SceneComponent.K2_SetWorldLocation` (`self.CollectableBase`) (`self.NewLocation`) false true)
      (set `self.ChangePlace` false)
      (set `/Game/Corregir/ThirdPerson/Blueprints/BP_TPC_NB_1.CollectablesBlue` (+ (`/Game/Corregir/ThirdPerson/Blueprints/BP_TPC_NB_1.CollectablesBlue` _asbp_tpc_nb_1) 1) _asbp_tpc_nb_1))
    (else
      (set `/Game/Corregir/ThirdPerson/Blueprints/BP_TPC_NR_2.CollectablesRed` 0 (stale `self.ColliderRojo.OnComponentBeginOverlap` _asbp_tpc_nr_2))
      (set `/Game/Corregir/ThirdPerson/Blueprints/BP_TPC_NB_1.CollectablesBlue` 0 _asbp_tpc_nb_1)
      (`SceneComponent.K2_SetWorldLocation` (`self.CollectableBase`) (`self.OldLocation`) false true)
      (set `self.ChangePlace` true))))

(event `self.ColliderRojo.OnComponentBeginOverlap`
  (params (OverlappedComponent :type "PrimitiveComponent Object Reference") (OtherActor :type "Actor Object Reference") (OtherComp :type "PrimitiveComponent Object Reference") (OtherBodyIndex :type Integer) (bFromSweep :type Boolean) (SweepResult :type "HitResult Structure (by ref)"))
  ;[1 1 1] Item Collection Red Ninja
  (bind _asbp_tpc_nr_2 (cast `/Game/Corregir/ThirdPerson/Blueprints/BP_TPC_NR_2` OtherActor))
  (if (`self.IsGreen`)
    (if (not (`self.ChangePlace`))
      (`SceneComponent.K2_SetWorldLocation` (`self.CollectableBase`) (`self.OldLocation`) false true)
      (set `self.ChangePlace` true)
      (bind _collectablesred (`/Game/Corregir/ThirdPerson/Blueprints/BP_TPC_NR_2.CollectablesRed` _asbp_tpc_nr_2))
      (set `/Game/Corregir/ThirdPerson/Blueprints/BP_TPC_NR_2.CollectablesRed` (+ _collectablesred 1) _asbp_tpc_nr_2)
      (if (>= _collectablesred 3)
        (`self.K2_DestroyActor`)))
    (else
      (set `/Game/Corregir/ThirdPerson/Blueprints/BP_TPC_NB_1.CollectablesBlue` 0 (stale `self.ColliderBlue.OnComponentBeginOverlap` _asbp_tpc_nb_1))
      (set `/Game/Corregir/ThirdPerson/Blueprints/BP_TPC_NR_2.CollectablesRed` 0 _asbp_tpc_nr_2)
      (`SceneComponent.K2_SetWorldLocation` (`self.CollectableBase`) (`self.OldLocation`) false true)
      (set `self.ChangePlace` true))))

(event `self.ReceiveTick`
  (params (DeltaSeconds :type "Float (single-precision)"))
  (bind _tintglass (`self.TintGlass`))
  ;[1 1 1] Color Change
  (`|ExecutionSequence`
    (:`then_0`
      (bind _output_get (set `self.Time` (+ DeltaSeconds (`self.Time`))))
      (if (>= _output_get 2.0)
        (set `self.Time` 0.0)
        (`|MultiGate` false true 0
          (:`Out 0`
            (`MaterialInstanceDynamic.SetVectorParameterValue` _tintglass "ColorBase" (`self.ColorVerde`))
            (set `self.IsGreen` true))
          (:`Out 1`
            (`MaterialInstanceDynamic.SetVectorParameterValue` _tintglass "ColorBase" (`self.ColorRojo`))
            (set `self.IsGreen` false)))))
    (:`then_1`
      ;[1 1 1] Rotation
      (`SceneComponent.K2_AddLocalRotation` (`self.Shuriken_low`) (`KismetMathLibrary.MakeRotator` 0.0 0.0 (* DeltaSeconds (`self.Velocity`))) false false))))

(fn `UserConstructionScript`)