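; BP_SpeedObj is a spinning collectable that temporarily raises the player character's blue collectable count.
; On overlap it increments CollectablesBlue, teleports itself aside and spawns a BPSpeedObj at a position offset from its starting relative location.
; After a delay it zeroes the count and returns to its stored location, using that relative position as a world position.
; Tick rotates the shuriken mesh and counts down ChangeDuration while collected.
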(event `self.ReceiveBeginPlay`
  (bind _relativelocation (`SceneComponent.RelativeLocation` (`self.CollectableBase`)))
  ;[1 1 1] Color Set and Specific Item
  (set `self.NextLocation` (+ _relativelocation (0.0 -1400.0 0.0)))
  (set `self.OldLocation` _relativelocation))

(event `self.Collider Blue.OnComponentBeginOverlap`
  (params (OverlappedComponent :type "PrimitiveComponent Object Reference") (OtherActor :type "Actor Object Reference") (OtherComp :type "PrimitiveComponent Object Reference") (OtherBodyIndex :type Integer) (bFromSweep :type Boolean) (SweepResult :type "HitResult Structure (by ref)"))
  ;[1 1 1] Item Collection
  (bind _asbp_tpc_nb_1 (cast `/Game/Corregir/ThirdPerson/Blueprints/BP_TPC_NB_1` OtherActor))
  (set `/Game/Corregir/ThirdPerson/Blueprints/BP_TPC_NB_1.CollectablesBlue` (+ (`/Game/Corregir/ThirdPerson/Blueprints/BP_TPC_NB_1.CollectablesBlue` _asbp_tpc_nb_1) 1) _asbp_tpc_nb_1)
  (`SceneComponent.K2_SetWorldLocation` (`self.CollectableBase`) (+ (`self.OldLocation`) (1000.0 0.0 0.0)) false true)
  (`|SpawnActorFromClass` (`self.BP_SpeedObj`) (`KismetMathLibrary.MakeTransform` (`self.NextLocation`)) "Undefined" "MultiplyWithRoot" null null)
  (`|ExecutionSequence`
    (:`then_0`
      (`KismetSystemLibrary.Delay` (`self.ChangeDuration`))
      (set `/Game/Corregir/ThirdPerson/Blueprints/BP_TPC_NB_1.CollectablesBlue` 0 _asbp_tpc_nb_1)
      (`SceneComponent.K2_SetWorldLocation` (`self.CollectableBase`) (`self.OldLocation`) false true)
      (set `self.changed?` false)
      (set `self.ChangeDuration` 3.0))
    (:`then_1`
      (set `self.changed?` true))))

(event `self.ReceiveTick`
  (params (DeltaSeconds :type "Float (single-precision)"))
  (bind _changeduration (`self.ChangeDuration`))
  ;[1 1 1] Countdown
  (`|ExecutionSequence`
    (:`then_0`
      (if (`self.changed?`)
        (set `self.ChangeDuration` (`KismetMathLibrary.FClamp` (- _changeduration DeltaSeconds) 0.0 _changeduration))))
    (:`then_1`
      ;[1 1 1] Rotation
      (`SceneComponent.K2_AddLocalRotation` (`self.Shuriken_low`) (`KismetMathLibrary.MakeRotator` 0.0 0.0 (* DeltaSeconds (`self.Velocity`))) false false))))

(fn `UserConstructionScript`)