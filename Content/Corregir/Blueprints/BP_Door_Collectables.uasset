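; BP_Door_Collectables is a sliding door with blue and red colliders, each responding to its own player character.
; Blue overlap plays the Timeline if CollectablesBlue meets CollectableCuantity; red overlap prints CollectablesRed and plays it without a threshold check.
; Each Timeline update adds MaxLocation scaled by DoorSlide to DoorC's current relative location with sweep, then zeroes both counters through the cast results from the two overlap events.
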(event `self.Collider Blue.OnComponentBeginOverlap`
  (params (OverlappedComponent :type "PrimitiveComponent Object Reference") (OtherActor :type "Actor Object Reference") (OtherComp :type "PrimitiveComponent Object Reference") (OtherBodyIndex :type Integer) (bFromSweep :type Boolean) (SweepResult :type "HitResult Structure (by ref)"))
  (bind _door_c (`self.Door_C`))
  ;[1 1 1] Collider Blue
  ;[1 1 1] Comprobador del personaje
  (bind _asbp_tpc_nb_1 (cast `/Game/Corregir/ThirdPerson/Blueprints/BP_TPC_NB_1` OtherActor))
  ;[1 1 1] Door Logic
  (if (>= (`/Game/Corregir/ThirdPerson/Blueprints/BP_TPC_NB_1.CollectablesBlue` _asbp_tpc_nb_1) (`self.CollectableCuantity`))
    ;[1 1 1] Set Location
    (bind (_direction _doorslide) (`Timeline|Timeline` :!label _label)
      (:`Update`
        (`SceneComponent.K2_SetRelativeLocation` _door_c (+ (`SceneComponent.RelativeLocation` _door_c) (* (`self.MaxLocation`) _doorslide)) true false)
        (`|ExecutionSequence`
          (:`then_0`
            (set `/Game/Corregir/ThirdPerson/Blueprints/BP_TPC_NB_1.CollectablesBlue` 0 _asbp_tpc_nb_1))
          (:`then_1`
            (set `/Game/Corregir/ThirdPerson/Blueprints/BP_TPC_NR_2.CollectablesRed` 0 (stale `self.Collider Red.OnComponentBeginOverlap` _asbp_tpc_nr_2))))))))

(event `self.Collider Red.OnComponentBeginOverlap`
  (params (OverlappedComponent :type "PrimitiveComponent Object Reference") (OtherActor :type "Actor Object Reference") (OtherComp :type "PrimitiveComponent Object Reference") (OtherBodyIndex :type Integer) (bFromSweep :type Boolean) (SweepResult :type "HitResult Structure (by ref)"))
  ;[1 1 1] Collider Red
  ;[1 1 1] Comprobador del personaje
  (bind _asbp_tpc_nr_2 (cast `/Game/Corregir/ThirdPerson/Blueprints/BP_TPC_NR_2` OtherActor))
  ;[1 1 1] Door Logic
  (bind _output_get (set `self.CollRed` (`/Game/Corregir/ThirdPerson/Blueprints/BP_TPC_NR_2.CollectablesRed` _asbp_tpc_nr_2)))
  (`KismetSystemLibrary.PrintString` (`KismetStringLibrary.Conv_IntToString` _output_get))
  (goto _label))

(fn `UserConstructionScript`)